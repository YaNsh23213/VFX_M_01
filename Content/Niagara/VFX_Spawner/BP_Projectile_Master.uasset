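; BP_Projectile_Master is a base VFX projectile that plays muzzle, flight and impact Niagara effects.
; Shortly after BeginPlay it spawns the muzzle effect at an offset from its location.
; Overlapping a BlockingVolume stops its movement, sets a Niagara bool to kill the main slash, spawns the impact effect and destroys the actor after a configurable delay.
; A shared SpawnVFX helper skips unset effects.
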(event OnComponentBeginOverlap(Projectile_collision_box)
  (params (OverlappedComponent :type Primitive%20Component%20Object%20Reference) (OtherActor :type Actor%20Object%20Reference) (OtherComp :type Primitive%20Component%20Object%20Reference) (OtherBodyIndex :type Integer) (bFromSweep :type Boolean) (SweepResult :type Hit%20Result%20Structure%20%28by%20ref%29))
  (Utilities|Casting|CastToBlockingVolume OtherActor)
  (Components|Movement|StopMovementImmediately (Variables|Default|GetProjectile_VFX_Movement_Comp))
  (Class|NiagaraComponent|SetVariableBool (Variables|Default|GetProjectile_VFX_Component) "ShouldKillMainSlash" true)
  (CallFunction|SpawnVFX (Variables|Default|GetHitImpactVFX) (Variables|Default|GetMuzzleHitImpactSpawnOffcet))
  (Utilities|FlowControl|Delay (Variables|Default|GetProjectile_destroy_delay))
  (Actor|DestroyActor))

(event EventBeginPlay
  (Utilities|FlowControl|Delay 0.1)
  (CallFunction|SpawnVFX (Variables|Default|GetMuzzleVFX) (Variables|Default|GetMuzzleHitImpactSpawnOffcet)))

(fn ConstructionScript)

(fn SpawnVFX
  (params (VFX%20to%20spawn :type Niagara%20System%20Object%20Reference) (SpawnOffcet :type Vector))
  (Utilities|IsValid VFX%20to%20spawn
    (:Is%20Valid
      (Niagara|SpawnSystematLocation VFX%20to%20spawn (+ SpawnOffcet (Transformation|GetActorLocation))))))